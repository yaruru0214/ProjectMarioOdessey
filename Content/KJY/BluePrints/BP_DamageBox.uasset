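; BP_DamageBox is an instant-kill hazard that sets Mario's HP in the game mode to zero when a Player-tagged actor hits it, guarded by a DoOnce.
; A non-Mario player, such as a possessed Goomba, is replaced by a spawned, possessed Mario for the death scene.
; Mario turns, input switches to UI-only, and the death montage's notify pauses the game, showing the game-over widget, cursor and reversed scene-change transition.
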(event `self.ReceiveBeginPlay`
  (bind _returnvalue (`GameplayStatics.GetActorOfClass` "/Game/KHH/BluePrints/BP_Goom.BP_Goom_C"))
  (set `self.MarioClone` _returnvalue)
  (bind _returnvalue_2 (`GameplayStatics.GetActorOfClass` "/Game/KHH/BluePrints/BP_Goom.BP_Goom_C"))
  (set `self.GoombaClone` _returnvalue_2))

(event `self.ReceiveHit`
  (params (MyComp :type "PrimitiveComponent Object Reference") (Other :type "Actor Object Reference") (OtherComp :type "PrimitiveComponent Object Reference") (bSelfMoved :type Boolean) (HitLocation :type "Vector Structure") (HitNormal :type "Vector Structure") (NormalImpulse :type "Vector Structure") (Hit :type "HitResult Structure (by ref)"))
  (bind (_returnvalue_location _returnvalue_rotation _returnvalue_scale) (`KismetMathLibrary.BreakTransform` (`self.GetTransform` Other)))
  ; 플레이어라면 닿을시 체력 0으로 세팅
  (`/Engine/EditorBlueprintResources/StandardMacros.DoOnce` false
    (:`Completed`
      (if (`self.ActorHasTag` Other "Player")
        (`self.MarioHPSet_0`)
        ; 게임오버파트
        (bind _asbp_game_mode_base (cast `/Game/KJY/BluePrints/BP_GameModeBase` (`GameplayStatics.GetGameMode`)))
        (if (<= (`/Game/KJY/BluePrints/BP_GameModeBase.MarioHP` _asbp_game_mode_base) 0)
          ; case 마리오
          (bind _asbp_mario (cast `/Game/KJY/BluePrints/BP_Mario` Other)
            (:`then`
              (bind _output_get (set `self.MarioDie` _asbp_mario))
              (bind (_returnvalue_roll _returnvalue_pitch _returnvalue_yaw) (`KismetMathLibrary.BreakRotator` (`KismetMathLibrary.FindLookAtRotation` (`self.K2_GetActorLocation` _asbp_mario) (`PlayerCameraManager.GetCameraLocation` (`PlayerController.PlayerCameraManager` (`GameplayStatics.GetPlayerController` 0))))))
              (`self.K2_SetActorRotation` _output_get (`KismetMathLibrary.MakeRotator` 0.0 0.0 (+ _returnvalue_yaw -90.0)) false))
            (:`CastFailed`
              ; case 굼바
              (bind _returnvalue (`|SpawnActorFromClass` "/Game/KJY/BluePrints/BP_Mario.BP_Mario_C" (`KismetMathLibrary.MakeTransform` (- _returnvalue_location (0.0 100.0 0.0)) _returnvalue_rotation _returnvalue_scale) "Undefined" "MultiplyWithRoot" null null))
              (`Controller.Possess` (`GameplayStatics.GetPlayerController` 0) _returnvalue)
              (bind _output_get_2 (set `self.MarioDie` _returnvalue))
              (bind (_returnvalue_roll_2 _returnvalue_pitch_2 _returnvalue_yaw_2) (`KismetMathLibrary.BreakRotator` (`self.K2_GetActorRotation` _output_get_2)))
              (`self.K2_SetActorRotation` _output_get_2 (`KismetMathLibrary.MakeRotator` 0.0 0.0 (+ _returnvalue_yaw_2 90.0)) false)))
          (`WidgetBlueprintLibrary.SetInputMode_UIOnlyEx` (`GameplayStatics.GetPlayerController` 0) null "DoNotLock" true)
          (`|PlayMontage` (`Character.Mesh` (`self.MarioDie`)) "/Game/Resource/Mario/Anim/Montage/MT_MarioDie.MT_MarioDie"
            (:`OnNotifyBegin`
              (bind _asbp_hud (cast `/Game/KHH/BluePrints/BP_HUD` (`PlayerController.GetHUD` (`GameplayStatics.GetPlayerController` 0))))
              (`Widget.SetVisibility` (`/Game/KHH/BluePrints/BP_HUD.WBP_GameOver` _asbp_hud) "Visible")
              (`GameplayStatics.SetGamePaused` true)
              (set `PlayerController.bShowMouseCursor` true (`GameplayStatics.GetPlayerController` 0))
              (bind _wbp_scenechange (`/Game/KHH/BluePrints/BP_HUD.WBP_SceneChange` _asbp_hud))
              (`|PlayAnimation` _wbp_scenechange (`/Game/KHH/UI/WBP_SceneChange.Shrink` _wbp_scenechange) 0.0 1 "Reverse"
                (:`Finished`
                  (`Widget.SetVisibility` _wbp_scenechange "Hidden"))))))))))

(fn `MarioHPSet_0`
  (bind _asbp_game_mode_base (cast `/Game/KJY/BluePrints/BP_GameModeBase` (`GameplayStatics.GetGameMode`)))
  (set `/Game/KJY/BluePrints/BP_GameModeBase.MarioHP` 0 _asbp_game_mode_base))

(fn `UserConstructionScript`)