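; AI controller for Goom that runs the BT_Goom behavior tree on possession and tracks the player through AI perception.
; Sensing an actor tagged Player cancels the forget timer and writes HasLineOfSight and Player to the Blackboard.
; Any other perception update, including non-player actors, starts a LineOfSightTimer delay that then clears both keys, giving a grace period before losing the player.
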(event `self.ReceivePossess`
  (params (PossessedPawn :type "Pawn Object Reference"))
  (`self.RunBehaviorTree` "/Game/KHH/AI/BT_Goom.BT_Goom"))

(event `self.AIPerception.OnTargetPerceptionUpdated`
  (params (Actor :type "Actor Object Reference") (Stimulus :type "AIStimulus Structure"))
  (bind _blackboard (`self.Blackboard`))
  (if (and (`self.ActorHasTag` Actor "Player") (`.bSuccessfullySensed` (break `AIStimulus` Stimulus)))
    (`KismetSystemLibrary.K2_ClearAndInvalidateTimerHandle` (`self.PlayerTimer`))
    (`BlackboardComponent.SetValueAsBool` _blackboard (`self.HasLineOfSight`) true)
    (`BlackboardComponent.SetValueAsObject` _blackboard (`self.Player`) Actor)
    (else
      (bind _returnvalue (`KismetSystemLibrary.K2_SetTimerDelegate` (delegate `StartPlayerTimer`) (`self.LineOfSightTimer`)))
      (set `self.PlayerTimer` _returnvalue))))

(event `StartPlayerTimer`
  (bind _blackboard (`self.Blackboard`))
  (`BlackboardComponent.SetValueAsBool` _blackboard (`self.HasLineOfSight`) false)
  (`BlackboardComponent.SetValueAsObject` _blackboard (`self.Player`) null))

(fn `UserConstructionScript`)