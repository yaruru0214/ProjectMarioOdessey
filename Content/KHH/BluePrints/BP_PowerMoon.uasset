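; BP_PowerMoon is the level goal pickup that starts the win sequence when Mario overlaps it.
; On overlap it disables its collision, turns Mario relative to the camera, plays his goal montage and switches input to UI only.
; A timeline lifts and spins the moon toward the camera.
; When the montage completes, the HUD shows the end and transition widgets, then pauses, shows the cursor and plays the win sound.
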(event `self.ReceiveBeginPlay`
  (set `self.Location` (`self.K2_GetActorLocation`)))

(event `self.ReceiveActorBeginOverlap`
  (params (OtherActor :type "Actor Object Reference"))
  (bind _returnvalue (`GameplayStatics.GetPlayerController` 0))
  (bind (_location_x _location_y _location_z) (`KismetMathLibrary.BreakVector` (`self.Location`)))
  (bind (_returnvalue_roll _returnvalue_pitch _returnvalue_yaw) (`KismetMathLibrary.BreakRotator` (`KismetMathLibrary.FindLookAtRotation` (`self.K2_GetActorLocation`) (`PlayerCameraManager.GetCameraLocation` (`PlayerController.PlayerCameraManager` (`GameplayStatics.GetPlayerController` 0))))))
  (bind _asbp_mario (cast `/Game/KJY/BluePrints/BP_Mario` OtherActor))
  (`PrimitiveComponent.SetCollisionEnabled` (`self.Box`) "NoCollision")
  (bind _output_get (set `self.BP_Mario` _asbp_mario))
  (bind (_returnvalue_roll_2 _returnvalue_pitch_2 _returnvalue_yaw_2) (`KismetMathLibrary.BreakRotator` (`KismetMathLibrary.FindLookAtRotation` (`self.K2_GetActorLocation` _output_get) (`PlayerCameraManager.GetCameraLocation` (`PlayerController.PlayerCameraManager` (`GameplayStatics.GetPlayerController` 0))))))
  (`self.K2_SetActorRotation` _output_get (`KismetMathLibrary.MakeRotator` 0.0 0.0 (+ _returnvalue_yaw_2 -80.0)) false)
  (`|PlayMontage` (`Character.Mesh` _output_get) "/Game/Resource/Mario/Anim/Montage/MT_MarioGoal.MT_MarioGoal" 1.0 0.0 "None" false
    (:`then`
      (`WidgetBlueprintLibrary.SetInputMode_UIOnlyEx` _returnvalue null "DoNotLock" true)
      (bind (_direction _moonup) (`Timeline|Timeline`)
        (:`Update`
          (`self.K2_SetActorLocation` (`KismetMathLibrary.MakeVector` _location_x _location_y (+ _location_z (* _moonup (`self.Size`)))))
          (`self.K2_SetActorRotation` (`KismetMathLibrary.MakeRotator` 0.0 0.0 (* _moonup (+ _returnvalue_yaw (* 360.0 (`self.StarRound`)))))))))
    (:`OnCompleted`
      (bind _asbp_hud (cast `/Game/KHH/BluePrints/BP_HUD` (`PlayerController.GetHUD` _returnvalue)))
      (`|ExecutionSequence`
        (:`then_0`
          (`Widget.SetVisibility` (`/Game/KHH/BluePrints/BP_HUD.WBP_End` _asbp_hud) "Visible")
          (bind _wbp_scenechange (`/Game/KHH/BluePrints/BP_HUD.WBP_SceneChange` _asbp_hud))
          (`Widget.SetVisibility` _wbp_scenechange "Visible"))
        (:`then_1`
          (`|PlayAnimation` _wbp_scenechange (`/Game/KHH/UI/WBP_SceneChange.Shrink` _wbp_scenechange) 0.0 1 "Reverse"
            (:`Finished`
              (`Widget.SetVisibility` _wbp_scenechange "Hidden")
              (`GameplayStatics.SetGamePaused` true)
              (set `PlayerController.bShowMouseCursor` true (`GameplayStatics.GetPlayerController` 0))
              (`GameplayStatics.PlaySound2D` "/Game/Resource/Sound/Bgm/SC_Win.SC_Win" 1.0 1.0 0.0 null null))))))))

(fn `UserConstructionScript`)