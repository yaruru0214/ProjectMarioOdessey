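; BP_Camera is a follow camera actor that becomes the player's view target when play begins.
; Each tick it moves to a fixed world-space offset behind and above the player pawn, then turns to face the pawn with a look-at rotation.
; The follow is rigid, with no interpolation, and the offset ignores the pawn's own rotation.
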(event `self.ReceiveBeginPlay`
  (`PlayerController.SetViewTargetWithBlend` (`GameplayStatics.GetPlayerController` 0) self 0.0 "VTBlend_Linear" 0.0 false))

(event `self.ReceiveTick`
  (params (DeltaSeconds :type "Float (single-precision)"))
  (bind (_returnvalue_x _returnvalue_y _returnvalue_z) (`KismetMathLibrary.BreakVector` (`self.K2_GetActorLocation` (`GameplayStatics.GetPlayerPawn` 0))))
  (`self.K2_SetActorLocation` (`KismetMathLibrary.MakeVector` (- _returnvalue_x 300.0) _returnvalue_y (+ _returnvalue_z 300.0)))
  (`self.K2_SetActorRotation` (`KismetMathLibrary.FindLookAtRotation` (`self.K2_GetActorLocation`) (`self.K2_GetActorLocation` (`GameplayStatics.GetPlayerPawn` 0)))))

(fn `UserConstructionScript`)