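; BP_ShirinkTile is a tile actor that sinks once the player has touched enough of its three sphere triggers.
; On BeginPlay it spawns a BP_SummonIcicle at each sphere's transform.
; Each player overlap disables that sphere's collision and increments Count through OverlapPlayer.
; When Count reaches FallCount, Tick waits out Delay, then moves the actor along its down vector at Speed for FallTime.
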(event `self.ReceiveBeginPlay`
  (bind (_returnvalue_location _returnvalue_rotation) (`KismetMathLibrary.BreakTransform` (`SceneComponent.K2_GetComponentToWorld` (`self.Sphere2`))))
  (bind (_returnvalue_location_2 _returnvalue_rotation_2) (`KismetMathLibrary.BreakTransform` (`SceneComponent.K2_GetComponentToWorld` (`self.Sphere`))))
  (bind (_returnvalue_location_3 _returnvalue_rotation_3) (`KismetMathLibrary.BreakTransform` (`SceneComponent.K2_GetComponentToWorld` (`self.Sphere1`))))
  (`|SpawnActorFromClass` "/Game/KHH/BluePrints/BP_SummonIcicle.BP_SummonIcicle_C" (`KismetMathLibrary.MakeTransform` _returnvalue_location_2 _returnvalue_rotation_2) "Undefined" "MultiplyWithRoot" null null)
  (`|SpawnActorFromClass` "/Game/KHH/BluePrints/BP_SummonIcicle.BP_SummonIcicle_C" (`KismetMathLibrary.MakeTransform` _returnvalue_location_3 _returnvalue_rotation_3) "Undefined" "MultiplyWithRoot" null null)
  (`|SpawnActorFromClass` "/Game/KHH/BluePrints/BP_SummonIcicle.BP_SummonIcicle_C" (`KismetMathLibrary.MakeTransform` _returnvalue_location _returnvalue_rotation) "Undefined" "MultiplyWithRoot" null null))

(event `self.ReceiveTick`
  (params (DeltaSeconds :type "Float (single-precision)"))
  (if (>= (`self.Count`) (`self.FallCount`))
    (bind _output_get (set `self.DelayTime` (+ (`self.DelayTime`) (`GameplayStatics.GetWorldDeltaSeconds`))))
    (if (> _output_get (`self.Delay`))
      (bind _output_get_2 (set `self.CurTime` (+ (`self.CurTime`) (`GameplayStatics.GetWorldDeltaSeconds`))))
      (if (< _output_get_2 (`self.FallTime`))
        (`self.K2_SetActorLocation` (+ (`self.K2_GetActorLocation`) (* (* (`self.GetActorUpVector`) -1.0) (`self.Speed`) (`GameplayStatics.GetWorldDeltaSeconds`))))))))

(event `self.Sphere.OnComponentBeginOverlap`
  (params (OverlappedComponent :type "PrimitiveComponent Object Reference") (OtherActor :type "Actor Object Reference") (OtherComp :type "PrimitiveComponent Object Reference") (OtherBodyIndex :type Integer) (bFromSweep :type Boolean) (SweepResult :type "HitResult Structure (by ref)"))
  (`self.OverlapPlayer` OtherActor (`self.Sphere`)))

(event `self.Sphere1.OnComponentBeginOverlap`
  (params (OverlappedComponent :type "PrimitiveComponent Object Reference") (OtherActor :type "Actor Object Reference") (OtherComp :type "PrimitiveComponent Object Reference") (OtherBodyIndex :type Integer) (bFromSweep :type Boolean) (SweepResult :type "HitResult Structure (by ref)"))
  (`self.OverlapPlayer` OtherActor (`self.Sphere1`)))

(event `self.Sphere2.OnComponentBeginOverlap`
  (params (OverlappedComponent :type "PrimitiveComponent Object Reference") (OtherActor :type "Actor Object Reference") (OtherComp :type "PrimitiveComponent Object Reference") (OtherBodyIndex :type Integer) (bFromSweep :type Boolean) (SweepResult :type "HitResult Structure (by ref)"))
  (`self.OverlapPlayer` OtherActor (`self.Sphere2`)))

(fn `OverlapPlayer`
  (params (Player :type "Actor Object Reference") (Target :type "PrimitiveComponent Object Reference"))
  (if (`self.ActorHasTag` Player "Player")
    (`PrimitiveComponent.SetCollisionEnabled` Target "NoCollision")
    (`/Engine/EditorBlueprintResources/StandardMacros.IncrementInt` (`self.Count`))))

(fn `UserConstructionScript`)