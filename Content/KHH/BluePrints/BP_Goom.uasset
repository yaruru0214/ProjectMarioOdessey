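; Goomba character that works as an AI monster or as a player-possessed body with movement, jump and pause input.
; Fire ejects a spawned BP_Mario and returns control to the AI; Mario landing on top destroys the Goomba.
; A player Goomba landing on a monster attaches to its head socket and possession moves to the lower one, building stacks.
; Other monster hits drain GameMode MarioHP with a cooldown, ending in Mario's death montage and game over.
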(event `self.ReceiveControllerChanged`
  (params (OldController :type "Controller Object Reference") (NewController :type "Controller Object Reference"))
  (bind `_as플레이어_컨트롤러` (cast `PlayerController` NewController))
  (bind _returnvalue (pcsubsystem `EnhancedInputLocalPlayerSubsystem` `_as플레이어_컨트롤러`))
  (`/Engine/EditorBlueprintResources/StandardMacros.IsValid` _returnvalue
    (:`Is Valid`
      _)
    (:`Is Not Valid`
      (message `EnhancedInputSubsystemInterface.AddMappingContext` _returnvalue "/Game/KJY/Inputs/IMC_Context.IMC_Context" 0 (struct))))
  (if (not (`self.IsChild`))
    (set `self.IsMonster` false)
    (`KismetArrayLibrary.Array_Add` (`self.Tags`) "Player")
    (set `self.bUseControllerRotationYaw` false)
    (`self.UpdateWalkSpeed` 500.0)))

(event `EnhancedInput|/Game/KJY/Inputs/IA_Jump`
  (params (ActionValue :type Boolean) (ElapsedSeconds :type "Float (double-precision)") (TriggeredSeconds :type "Float (double-precision)") (InputAction :type "InputAction Object Reference" :default "/Game/KJY/Inputs/IA_Jump.IA_Jump"))
  (:`Started`
    (`self.Jump`)))

(event `EnhancedInput|/Game/KJY/Inputs/IA_Fire`
  (params (ActionValue :type Boolean) (ElapsedSeconds :type "Float (double-precision)") (TriggeredSeconds :type "Float (double-precision)") (InputAction :type "InputAction Object Reference" :default "/Game/KJY/Inputs/IA_Fire.IA_Fire"))
  (bind _goomaicontroller (`self.GoomAIController`))
  (:`Started`
    (bind _returnvalue (`|SpawnActorFromClass` "/Game/KJY/BluePrints/BP_Mario.BP_Mario_C" (`SceneComponent.K2_GetComponentToWorld` (`self.Arrow1`)) "Undefined" "MultiplyWithRoot" null null))
    (`Controller.Possess` (`GameplayStatics.GetPlayerController` 0) _returnvalue)
    (set `self.IsMonster` true)
    (`KismetArrayLibrary.Array_RemoveItem` (`self.Tags`) "Player")
    (`/Engine/EditorBlueprintResources/StandardMacros.IsValid` _goomaicontroller
      (:`Is Valid`
        (`Controller.Possess` _goomaicontroller self)))))

(event `EnhancedInput|/Game/KJY/Inputs/IA_Look`
  (params (ActionValue :type "Vector2D Structure") (ElapsedSeconds :type "Float (double-precision)") (TriggeredSeconds :type "Float (double-precision)") (InputAction :type "InputAction Object Reference" :default "/Game/KJY/Inputs/IA_Look.IA_Look"))
  (:`Triggered`
    (`self.AddControllerYawInput` ActionValue_X)
    (`self.AddControllerPitchInput` ActionValue_Y)))

(event `EnhancedInput|/Game/KJY/Inputs/IA_WASD`
  (params (ActionValue :type "Vector Structure") (ElapsedSeconds :type "Float (double-precision)") (TriggeredSeconds :type "Float (double-precision)") (InputAction :type "InputAction Object Reference" :default "/Game/KJY/Inputs/IA_WASD.IA_WASD"))
  (bind (_returnvalue_roll _returnvalue_pitch _returnvalue_yaw) (`KismetMathLibrary.BreakRotator` (`self.GetControlRotation`)))
  (bind (_returnvalue_roll_2 _returnvalue_pitch_2 _returnvalue_yaw_2) (`KismetMathLibrary.BreakRotator` (`self.GetControlRotation`)))
  (:`Triggered`
    (`self.AddMovementInput` (`KismetMathLibrary.GetRightVector` (`KismetMathLibrary.MakeRotator` _returnvalue_roll_2 0.0 _returnvalue_yaw_2)) ActionValue_X)
    (`self.AddMovementInput` (`KismetMathLibrary.GetForwardVector` (`KismetMathLibrary.MakeRotator` 0.0 0.0 _returnvalue_yaw)) ActionValue_Y)))

(event `EnhancedInput|/Game/KJY/Inputs/IA_Menu`
  (params (ActionValue :type Boolean) (ElapsedSeconds :type "Float (double-precision)") (TriggeredSeconds :type "Float (double-precision)") (InputAction :type "InputAction Object Reference" :default "/Game/KJY/Inputs/IA_Menu.IA_Menu"))
  (bind _returnvalue (`GameplayStatics.GetPlayerController` 0))
  (:`Started`
    (bind _asbp_hud (cast `/Game/KHH/BluePrints/BP_HUD` (`PlayerController.GetHUD` (`GameplayStatics.GetPlayerController` 0))))
    (`Widget.SetVisibility` (`/Game/KHH/BluePrints/BP_HUD.WBP_Pause` _asbp_hud) "Visible")
    (`GameplayStatics.SetGamePaused` true)
    (set `PlayerController.bShowMouseCursor` true _returnvalue)
    (`WidgetBlueprintLibrary.SetInputMode_UIOnlyEx` _returnvalue null)))

(event `self.ReceiveBeginPlay`
  (bind _asbp_goom_controller (cast `/Game/KHH/AI/BP_GoomController` (`AIBlueprintHelperLibrary.GetAIController` self)))
  (set `self.GoomAIController` _asbp_goom_controller)
  (bind _asbp_game_mode_base (cast `/Game/KJY/BluePrints/BP_GameModeBase` (`GameplayStatics.GetGameMode`)))
  (set `self.BPGameModeBase` _asbp_game_mode_base))

(event `self.ReceiveTick`
  (params (DeltaSeconds :type "Float (single-precision)")))

(event `self.ReceiveHit`
  (params (MyComp :type "PrimitiveComponent Object Reference") (Other :type "Actor Object Reference") (OtherComp :type "PrimitiveComponent Object Reference") (bSelfMoved :type Boolean) (HitLocation :type "Vector Structure") (HitNormal :type "Vector Structure") (NormalImpulse :type "Vector Structure") (Hit :type "HitResult Structure (by ref)"))
  (bind _returnvalue (`GameplayStatics.GetPlayerController` 0))
  (bind _z (.z HitNormal))
  (bind _bpgamemodebase (`self.BPGameModeBase`))
  (if (not (`self.IsChild`))
    (bind _asbp_mario (cast `/Game/KJY/BluePrints/BP_Mario` Other)
      (:`then`
        (if (< _z -0.5)
          (`self.LaunchCharacter` _asbp_mario (`self.GetActorForwardVector` _asbp_mario) false false)
          (`self.K2_DestroyActor`)))
      (:`CastFailed`
        (bind _asbp_goom (cast `/Game/KHH/BluePrints/BP_Goom` Other))
        (if (`/Game/KHH/BluePrints/BP_Goom.IsMonster` _asbp_goom)
          (if (`self.ActorHasTag` "Player")
            (if (> _z 0.5)
              (`|ExecutionSequence`
                (:`then_0`
                  (`self.K2_SetActorRotation` _asbp_goom (`self.K2_GetActorRotation`) false)
                  (`self.K2_AttachToComponent` (`Character.Mesh` _asbp_goom) "HeadSo" "SnapToTarget" "SnapToTarget" "KeepWorld")
                  (`KismetArrayLibrary.Array_RemoveItem` (`self.Tags`) "Player")
                  (set `self.IsChild` true)
                  (`SceneComponent.K2_SetRelativeRotation` (`self.Mesh`) (struct :`Pitch` -90.0 :`Roll` -90.0) false false))
                (:`then_1`
                  (`Controller.Possess` (`GameplayStatics.GetPlayerController` 0) _asbp_goom)
                  (set `/Game/KHH/BluePrints/BP_Goom.IsMonster` false _asbp_goom)
                  (set `/Game/KHH/BluePrints/BP_Goom.IsRoot` true _asbp_goom)
                  (`PrimitiveComponent.SetCollisionEnabled` (`self.CapsuleComponent`) "NoCollision")))
              (elif (`self.CanDamage`)
                (bind _output_get (set `/Game/KJY/BluePrints/BP_GameModeBase.MarioHP` (- (`/Game/KJY/BluePrints/BP_GameModeBase.MarioHP` _bpgamemodebase) 1) _bpgamemodebase))
                (if (> _output_get 0)
                  (set `self.CanDamage` false)
                  (`KismetSystemLibrary.Delay` 3.0)
                  (set `self.CanDamage` true)
                  (else
                    (bind _returnvalue_2 (`|SpawnActorFromClass` "/Game/KJY/BluePrints/BP_Mario.BP_Mario_C" (`SceneComponent.K2_GetComponentToWorld` (`self.Arrow1`)) "Undefined" "MultiplyWithRoot" null null))
                    (`Controller.Possess` (`GameplayStatics.GetPlayerController` 0) _returnvalue_2)
                    (bind _output_get_2 (set `self.MarioDie` _returnvalue_2))
                    (bind (_returnvalue_roll _returnvalue_pitch _returnvalue_yaw) (`KismetMathLibrary.BreakRotator` (`KismetMathLibrary.FindLookAtRotation` (`self.K2_GetActorLocation` _output_get_2) (`PlayerCameraManager.GetCameraLocation` (`PlayerController.PlayerCameraManager` (`GameplayStatics.GetPlayerController` 0))))))
                    (`self.K2_SetActorRotation` _output_get_2 (`KismetMathLibrary.MakeRotator` 0.0 0.0 (+ _returnvalue_yaw -90.0)) false)
                    (`|PlayMontage` (`Character.Mesh` (`self.MarioDie`)) "/Game/Resource/Mario/Anim/Montage/MT_MarioDie.MT_MarioDie"
                      (:`OnCompleted`
                        (bind _asbp_hud (cast `/Game/KHH/BluePrints/BP_HUD` (`PlayerController.GetHUD` (`GameplayStatics.GetPlayerController` 0))))
                        (`Widget.SetVisibility` (`/Game/KHH/BluePrints/BP_HUD.WBP_GameOver` _asbp_hud) "Visible")
                        (`GameplayStatics.SetGamePaused` true)
                        (`WidgetBlueprintLibrary.SetInputMode_UIOnlyEx` _returnvalue null "DoNotLock" true)
                        (set `PlayerController.bShowMouseCursor` true _returnvalue)))))))))))))

(fn `UpdateWalkSpeed`
  (params (NewWalkSpeed :type "Float (double-precision)"))
  (set `CharacterMovementComponent.MaxWalkSpeed` NewWalkSpeed (`self.CharacterMovement`)))

(fn `UserConstructionScript`)